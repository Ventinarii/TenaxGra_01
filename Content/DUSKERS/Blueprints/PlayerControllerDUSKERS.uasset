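; Player controller for DUSKERS that captures mouse and keyboard input and rebroadcasts it through event dispatchers.
; Mouse buttons and wheel directions each fire their own call, while a handful of letter keys and Left Alt share one KeyEvent call carrying the key and its down state.
; An unconnected leftover chain adds a widget to the viewport and caches the flying camera pawn, but it never runs.
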(event `self.ReceiveBeginPlay`)

(event `Key|LeftMouseButton`
  (params (Key :type "Key Structure"))
  (:`Pressed`
    (`self.LeftMouseButtonDown`))
  (:`Released`
    (`self.LeftMouseButtonUp`)))

(event `Key|RightMouseButton`
  (params (Key :type "Key Structure"))
  (:`Pressed`
    (`self.RightMouseButtonDown`))
  (:`Released`
    (`self.RightMouseButtonUp`)))

(event `Key|MouseScrollUp`
  (params (Key :type "Key Structure"))
  (:`Pressed`
    (`self.MouseWheelUp`)))

(event `Key|MouseScrollDown`
  (params (Key :type "Key Structure"))
  (:`Pressed`
    (`self.MouseWheelDown`)))

(event `Key|M`
  (params (Key :type "Key Structure"))
  (:`Pressed`
    (`self.KeyEvent` Key true))
  (:`Released`
    (`self.KeyEvent` Key)))

(event `Key|S`
  (params (Key :type "Key Structure"))
  (:`Pressed`
    (`self.KeyEvent` Key true))
  (:`Released`
    (`self.KeyEvent` Key)))

(event `Key|H`
  (params (Key :type "Key Structure"))
  (:`Pressed`
    (`self.KeyEvent` Key true))
  (:`Released`
    (`self.KeyEvent` Key)))

(event `Key|P`
  (params (Key :type "Key Structure"))
  (:`Pressed`
    (`self.KeyEvent` Key true))
  (:`Released`
    (`self.KeyEvent` Key)))

(event `Key|A`
  (params (Key :type "Key Structure"))
  (:`Pressed`
    (`self.KeyEvent` Key true))
  (:`Released`
    (`self.KeyEvent` Key)))

(event `Key|LeftAlt`
  (params (Key :type "Key Structure"))
  (:`Pressed`
    (`self.KeyEvent` Key true))
  (:`Released`
    (`self.KeyEvent` Key)))

(fn `UserConstructionScript`)