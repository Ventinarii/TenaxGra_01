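; Metagame map actor that switches between a galaxy view of all maps and a local view of the selected map's locations.
; Construction and BeginPlay share one refresh that clamps selection indices, sets visibility and background material, and snaps the ship to the selection, so editor changes preview immediately.
; Events add maps or locations, remove maps and send the ship to the selection.
; GetDistanceTo measures to a target in the active view, returning -1 when invalid.
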(event `self.ReceiveBeginPlay`
  (bind _staticmesh (`self.StaticMesh`))
  (bind _maps (`self.Maps`))
  (bind _maps_2 (`self.Maps`))
  (bind _selectedmap (`self.SelectedMap`))
  (bind _mymetaspaceship (`self.MyMetaSpaceShip`))
  (bind _maps_3 (`self.Maps`))
  (bind _returnvalue (`KismetArrayLibrary.Array_Length` _maps_3))
  (bind _returnvalue_2 (`KismetArrayLibrary.Array_Length` (`/Game/DUSKERS/Blueprints/MetaGame/MyMetaLocationActor.LocationMap` (`|GetArrayItem` _maps_3 _selectedmap))))
  (`|ExecutionSequence` :!label _label
    (:`then_0`
      ;[1 1 1] Data validation
      (if (<= _returnvalue _selectedmap)
        (set `self.SelectedMap` (- _returnvalue 1)))
      (if (!= _returnvalue 0)
        (if (<= _returnvalue_2 (`self.SelectLocation`))
          (set `self.SelectLocation` (- _returnvalue_2 1)))
        (else
          (set `self.SelectLocation` -1))))
    (:`then_1`
      (if (`self.ShowGalaxyMap`)
        (`|ExecutionSequence` :!label _label_2
          (:`then_0`
            ;[1 1 1] Set visibility of galaxy map & hide locs
            (for _array_element _maps_2
              (`SceneComponent.SetVisibility` (`/Game/DUSKERS/Blueprints/MetaGame/MyMetaLocationActor.DefaultSceneRoot` _array_element) true true)
              (`/Game/DUSKERS/Blueprints/MetaGame/MyMetaLocationActor.SetLocVisible` _array_element false)))
          (:`then_1`
            ;[1 1 1] Set Material on jump/action
            (`PrimitiveComponent.SetMaterial` _staticmesh 0 "/Game/DUSKERS/Blueprints/MetaGame/Materials/GalaxyMap_Mat.GalaxyMap_Mat")))
        (else
          (`|ExecutionSequence` :!label _label_3
            (:`then_0`
              (for _array_element_2 _maps_2
                (`SceneComponent.SetVisibility` (`Actor.RootComponent` _array_element_2) false true)
                (`/Game/DUSKERS/Blueprints/MetaGame/MyMetaLocationActor.SetLocVisible` _array_element_2 false))
              ;[1 1 1] Show correct locs
              (if (!= (`KismetArrayLibrary.Array_Length` _maps) 0)
                (`/Game/DUSKERS/Blueprints/MetaGame/MyMetaLocationActor.SetLocVisible` (`|GetArrayItem` _maps (`self.SelectedMap`)) true)))
            (:`then_1`
              (if (== (`self.SelectedMap`) -1)
                (`PrimitiveComponent.SetMaterial` _staticmesh 0 "/Game/DUSKERS/Blueprints/MetaGame/Materials/UniwerseMap_Mat.UniwerseMap_Mat")
                (else
                  (`PrimitiveComponent.SetMaterial` _staticmesh 0 (`/Game/DUSKERS/Blueprints/MetaGame/MyMetaLocationActor.Background` (`|GetArrayItem` (`self.Maps`) (`self.SelectedMap`)))))))))))
    (:`then_2`
      ;[1 1 1] teleport/move to loc on edit / game start / command
      (if (`self.ShowGalaxyMap`)
        (if (!= (`self.SelectedMap`) -1)
          (`SceneComponent.K2_SetWorldLocation` _mymetaspaceship (`SceneComponent.K2_GetComponentLocation` (`/Game/DUSKERS/Blueprints/MetaGame/MyMetaLocationActor.DefaultSceneRoot` (`|GetArrayItem` (`self.Maps`) (`self.SelectedMap`)))) false false))
        (elif (!= (`self.SelectLocation`) -1)
          (`SceneComponent.K2_SetWorldLocation` _mymetaspaceship (`SceneComponent.K2_GetComponentLocation` (`/Game/DUSKERS/Blueprints/MetaGame/MyMetaLocationActor.DefaultSceneRoot` (`|GetArrayItem` (`/Game/DUSKERS/Blueprints/MetaGame/MyMetaLocationActor.LocationMap` (`|GetArrayItem` (`self.Maps`) (`self.SelectedMap`))) (`self.SelectLocation`)))) false false))))))

(event `ContructionEvent`
  (goto _label))

(event `SetVisibility`
  (params (ShowGalaxyMap :type Boolean))
  (if (not (== ShowGalaxyMap (`self.ShowGalaxyMap`)))
    (set `self.ShowGalaxyMap` ShowGalaxyMap)
    (if ShowGalaxyMap
      (goto _label_2)
      (else
        (goto _label_3)))))

(event `MoveToLocFromUI`
  ;[1 1 1] teleport/move to loc on edit / game start / command
  (bind _asmy_meta_space_ship (cast `/Game/DUSKERS/Blueprints/MetaGame/MyMetaSpaceShip` (`ChildActorComponent.ChildActor` (`self.MyMetaSpaceShip`))))
  (if (`self.ShowGalaxyMap`)
    (if (!= (`self.SelectedMap`) -1)
      (`/Game/DUSKERS/Blueprints/MetaGame/MyMetaSpaceShip.SimpleMoveToLoc` _asmy_meta_space_ship (`SceneComponent.K2_GetComponentLocation` (`/Game/DUSKERS/Blueprints/MetaGame/MyMetaLocationActor.DefaultSceneRoot` (`|GetArrayItem` (`self.Maps`) (`self.SelectedMap`))))))
    (elif (!= (`self.SelectLocation`) -1)
      (`/Game/DUSKERS/Blueprints/MetaGame/MyMetaSpaceShip.SimpleMoveToLoc` _asmy_meta_space_ship (`SceneComponent.K2_GetComponentLocation` (`/Game/DUSKERS/Blueprints/MetaGame/MyMetaLocationActor.DefaultSceneRoot` (`|GetArrayItem` (`/Game/DUSKERS/Blueprints/MetaGame/MyMetaLocationActor.LocationMap` (`|GetArrayItem` (`self.Maps`) (`self.SelectedMap`))) (`self.SelectLocation`))))))))

(event `AddNewLocation`
  ;[1 1 1] Add new location and show it
  (if (== (`self.SelectedMap`) -1)
    (`self.AddNewMap`)
    (set `self.SelectedMap` 0)
    (else
      (`/Game/DUSKERS/Blueprints/MetaGame/MyMetaLocationActor.AddNewLocation` (`|GetArrayItem` (`self.Maps`) (`self.SelectedMap`)))))
  (`self.SetVisibility` false))

(event `AddNewMap`
  ;[1 1 1] Create and add new map in galaxy view
  (`self.SetVisibility` true)
  (bind _returnvalue (`|SpawnActorFromClass` "/Game/DUSKERS/Blueprints/MetaGame/MyMetaLocationActor.MyMetaLocationActor_C" (`self.GetTransform`) "Undefined" "OverrideRootScale" null "NewMap" self true null null))
  (`KismetArrayLibrary.Array_Add` (`self.Maps`) _returnvalue))

(event `RemoveMap`
  (params (ToRemove :type "/Game/DUSKERS/Blueprints/MetaGame/MyMetaLocationActor Object Reference (by ref)"))
  (bind _returnvalue (`KismetArrayLibrary.Array_RemoveItem` (`self.Maps`) ToRemove))
  (if _returnvalue
    (`self.K2_DestroyActor` ToRemove)))

(fn `Get Distance To`
  (params (Target :type Integer))
  (returns (Distance :type "Float (double-precision)") (IsGalaxyMap :type Boolean))
  (bind _locationmap (`/Game/DUSKERS/Blueprints/MetaGame/MyMetaLocationActor.LocationMap` (`|GetArrayItem` (`self.Maps`) (`self.SelectedMap`))))
  (if (and (!= (`self.SelectedMap`) -1) (!= (`self.SelectLocation`) -1) (select `bool` (`self.ShowGalaxyMap`) :`false` true :`true` (< Target (`KismetArrayLibrary.Array_Length` (`self.Maps`)))))
    (if (`self.ShowGalaxyMap`)
      (return (`self.GetDistanceTo` (`|GetArrayItem` (`self.Maps`) (`self.SelectedMap`)) (`|GetArrayItem` (`self.Maps`) Target)) true)
      (elif (< Target (`KismetArrayLibrary.Array_Length` _locationmap))
        (return (`self.GetDistanceTo` (`|GetArrayItem` _locationmap (`self.SelectLocation`)) (`|GetArrayItem` _locationmap Target)) false)
        (else
          _))))
  (return -1.0 (`self.ShowGalaxyMap`)) ; data invalid - error
)

(fn `UserConstructionScript`
  (`self.ContructionEvent`))