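; MyMetaLocationActor is a meta-game map node that forms a tree of locations through its LocationMap array.
; AddNewLocation spawns child nodes of the same class at the owning system's transform, with itself as owner.
; DeleteSystem requests removal from the system or location owner, depending on IsGalaxyMap.
; SetLocVisible propagates visibility to children, and Destroyed cascades destruction down the tree.
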(event `DeleteSystem`
  (if (`self.IsGalaxyMap`)
    (`/Game/DUSKERS/Blueprints/MetaGame/MyMetaMap.RemoveMap` (`self.OwnerOfSys`) self)
    (else
      (`self.RemoveLocation` (`self.OwnerOfLoc`) self))))

(event `self.ReceiveDestroyed`
  (for _array_element (`self.LocationMap`)
    (`self.K2_DestroyActor` _array_element)))

(event `SetLocVisible`
  (params (Visible :type Boolean))
  (for _array_element (`self.LocationMap`)
    (`SceneComponent.SetVisibility` (`Actor.RootComponent` _array_element) Visible true)))

(event `AddNewLocation`
  (bind _returnvalue (`|SpawnActorFromClass` "MyMetaLocationActor_C" (`self.GetTransform` (`self.OwnerOfSys`)) "Undefined" "OverrideRootScale" null "NewMap" null false self null))
  (`KismetArrayLibrary.Array_Add` (`self.LocationMap`) _returnvalue))

(event `RemoveLocation`
  (params (ToRemove :type "/Game/DUSKERS/Blueprints/MetaGame/MyMetaLocationActor Object Reference (by ref)"))
  (bind _returnvalue (`KismetArrayLibrary.Array_RemoveItem` (`self.LocationMap`)))
  (if _returnvalue
    (`self.K2_DestroyActor`)))

(fn `UserConstructionScript`)