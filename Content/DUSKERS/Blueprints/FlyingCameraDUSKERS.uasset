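; Flying camera for DUSKERS with drag panning, wheel zoom, numpad rotation and a surface-aligned, colour-switchable decal cursor.
; A looping timer places the cursor under the mouse, eases zoom and moves the Billboard toward the grabbed ground-plane point, capped by Speed.
; PlayerControllerDUSKERS delegates drive left-drag (Shift excluded for unit selection) and zoom.
; Numpad 8/2/4/6 play two timelines that tilt and swing the view, reversing on release.
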(event `self.ReceiveBeginPlay`
  (bind (_x _y) (`KismetMathLibrary.BreakVector2D` (`WidgetLayoutLibrary.GetViewportSize`)))
  (`|ExecutionSequence`
    (:`then_0`
      (set `self.TargetPosition` (.location (`SceneComponent.GetRelativeTransform` (`self.Camera`)))))
    (:`then_1`
      (`self.ChangeCursor` "NewEnumerator6"))
    (:`then_2`
      (`ActorComponent.SetActive` (`self.Camera`) true false)
      (`KismetSystemLibrary.K2_SetTimerDelegate` (delegate `HandleCamMovement`) 0.01 true)
      (set `self.ScreenRX` (- _x 100.0))
      (set `self.ScreenTY` (- _y 100.0))
      (`SceneComponent.K2_SetWorldTransform` (`self.Billboard`) (`KismetMathLibrary.MakeTransform` (0.0 0.0 500.0)) false false))
    (:`then_3`
      (bind _asplayer_controller_duskers (cast `/Game/DUSKERS/Blueprints/PlayerControllerDUSKERS` (`GameplayStatics.GetPlayerController` 0)))
      (add `/Game/DUSKERS/Blueprints/PlayerControllerDUSKERS.LeftMouseButtonDown` _asplayer_controller_duskers (delegate `LMB-Down`))
      (add `/Game/DUSKERS/Blueprints/PlayerControllerDUSKERS.LeftMouseButtonUp` _asplayer_controller_duskers (delegate `LMB-UP`))
      (add `/Game/DUSKERS/Blueprints/PlayerControllerDUSKERS.MouseWheelUp` _asplayer_controller_duskers (delegate `MW-UP`))
      (add `/Game/DUSKERS/Blueprints/PlayerControllerDUSKERS.MouseWheelDown` _asplayer_controller_duskers (delegate `MW-DOWN`)))))

(event `HandleCamMovement`
  (bind _speed (`self.Speed`))
  (bind (_worldlocation _worlddirection) (`PlayerController.DeprojectMousePositionToWorld` (`GameplayStatics.GetPlayerController` 0)))
  (bind _location (.location (`SceneComponent.GetRelativeTransform` (`self.Camera`))))
  (bind (_bblockinghit _binitialoverlap _time _distance _location_2 _impactpoint _normal) (`GameplayStatics.BreakHitResult` (`PlayerController.GetHitResultUnderCursorByChannel` (`GameplayStatics.GetPlayerController` 0) "TraceTypeQuery1" true)))
  (bind _returnvalue (- _location (`self.TargetPosition`)))
  (bind _returnvalue_2 (* (- (`self.GrabedWorldLocation`) (+ _worldlocation (* (* _worlddirection (`KismetMathLibrary.SafeDivide` (.z _worldlocation) (.z _worlddirection))) -1.0))) 0.05))
  (bind _returnvalue_3 (`KismetMathLibrary.VSize` _returnvalue_2))
  ;[1 1 1] Move camera in world
  (`|ExecutionSequence`
    (:`then_0`
      ;;[1 1 1] Mouse Cursor
      (`SceneComponent.K2_SetWorldLocationAndRotation` (`self.Cursor`) _location_2 (`KismetMathLibrary.MakeRotationFromAxes` _normal) false false))
    (:`then_1`
      ;;[1 1 1] smooth zoom
      (if (> (`KismetMathLibrary.VSize` _returnvalue) 1.0)
        (`SceneComponent.K2_SetRelativeLocation` (`self.Camera`) (+ (* _returnvalue -0.05) _location) false false)))
    (:`then_2`
      ;;[1 1 1] smooth Move camera to grab
      (if (`self.IsRightMouseButtonPressed`)
        (`SceneComponent.K2_AddLocalOffset` (`self.Billboard`) (select `bool` (< _returnvalue_3 _speed) :`false` (/ _returnvalue_2 (/ _returnvalue_3 _speed)) :`true` _returnvalue_2) false false)))))

(event `ChangeCursor`
  (params (CursorState :type "/Game/DUSKERS/MaterialsLearning/Cursors/CursorColor Enum" :default "NewEnumerator0"))
  (bind _cursor (`self.Cursor`))
  ;[1 1 1] Move camera in world
  ;;[1 1 1] Mouse Cursor
  (`DecalComponent.SetDecalMaterial` _cursor (select `/Game/DUSKERS/MaterialsLearning/Cursors/CursorColor` CursorState :`NewEnumerator0` "/Game/DUSKERS/MaterialsLearning/Cursors/Cursor_R.Cursor_R" :`NewEnumerator1` "/Game/DUSKERS/MaterialsLearning/Cursors/Cursor_G.Cursor_G" :`NewEnumerator2` "/Game/DUSKERS/MaterialsLearning/Cursors/Cursor_G.Cursor_G" :`NewEnumerator3` "/Game/DUSKERS/MaterialsLearning/Cursors/Cursor_B.Cursor_B" :`NewEnumerator4` "/Game/DUSKERS/MaterialsLearning/Cursors/Cursor_M.Cursor_M" :`NewEnumerator5` "/Game/DUSKERS/MaterialsLearning/Cursors/Cursor_Y.Cursor_Y" :`NewEnumerator6` "/Game/DUSKERS/MaterialsLearning/Cursors/Cursor.Cursor" :`NewEnumerator7` "/Game/DUSKERS/MaterialsLearning/Cursors/Cursor.Cursor" :!type "MaterialInterface Object Reference"))
  (`SceneComponent.SetVisibility` _cursor (`|EnumEquality` CursorState "NewEnumerator7") false))

(event `LMB-Down`
  (bind (_worldlocation _worlddirection) (`PlayerController.DeprojectMousePositionToWorld` (`GameplayStatics.GetPlayerController` 0)))
  ;[1 1 1] Move camera in world
  ;;[1 1 1] Grab world
  (if (not (`PlayerController.IsInputKeyDown` (`GameplayStatics.GetPlayerController` 0) "LeftShift"))
    (set `self.IsRightMouseButtonPressed` true)
    (set `self.GrabedWorldLocation` (+ _worldlocation (* (* _worlddirection (`KismetMathLibrary.SafeDivide` (.z _worldlocation) (.z _worlddirection))) -1.0)))))

(event `LMB-UP`
  ;[1 1 1] Move camera in world
  ;;[1 1 1] Grab world
  (set `self.IsRightMouseButtonPressed` false))

(event `MW-UP`
  (bind _zoomspeed (`self.ZoomSpeed`))
  (bind _targetposition (`self.TargetPosition`))
  ;[1 1 1] Move camera in world
  ;;[1 1 1] Camera control
  (`/Engine/EditorBlueprintResources/StandardMacros.CompareFloat` (.x _targetposition) -1.0
    (:`>`
      (set `self.TargetPosition` (0.0 0.0 0.0)))
    (:`<`
      (set `self.TargetPosition` (+ (* (`KismetMathLibrary.MakeVector` (* _zoomspeed -1.0) _zoomspeed _zoomspeed) -1) _targetposition)))))

(event `MW-DOWN`
  (bind _zoomspeed (`self.ZoomSpeed`))
  (bind _targetposition (`self.TargetPosition`))
  ;[1 1 1] Move camera in world
  ;;[1 1 1] Camera control
  (`/Engine/EditorBlueprintResources/StandardMacros.CompareFloat` (.x _targetposition) (`self.ZoomTop`)
    (:`>`
      (set `self.TargetPosition` (+ (`KismetMathLibrary.MakeVector` (* _zoomspeed -1.0) _zoomspeed _zoomspeed) _targetposition)))
    (:`<`
      (set `self.TargetPosition` (-4000.0 4000.0 4000.0)))))

(event `Key|NumPadEight`
  (params (Key :type "Key Structure"))
  (bind _returnvalue (`GameplayStatics.GetPlayerController` 0))
  (bind _camera (`self.Camera`))
  (bind _yaw (.yaw (.rotation (`SceneComponent.GetRelativeTransform` _camera))))
  ;[1 1 1] Camera rotation (not perfect but good enough)
  ;;[1 1 1] Camera Up and Down rotation
  (:`Pressed`
    (if (not (`self.CamRotDown`)) :!label _label
      (set `self.CamRotUp` true)
      (bind (_direction _from_0_to_1_in_2_sec) (`Timeline|CamRotTimelineYAxis` :!label _label_2)
        (:`Update`
          ;;[1 1 1] Check if movement is exclusive
          (if (or (`self.CamRotLeft`) (`self.CamRotRight`))
            ;;[1 1 1] Apply movment
            (if (`self.CamRotLeft`) :!label _label_3
              (if (`self.CamRotUp`)
                (bind _returnvalue_2 (- (* _from_0_to_1_in_2_sec 45.0) 45.0))
                (bind _returnvalue_3 (- (* (stale `Key|NumPadFour` _from_0_to_1_in_2_sec) -45.0) 45.0))
                (`SceneComponent.K2_SetRelativeRotation` _camera (`KismetMathLibrary.MakeRotator` 0.0 _returnvalue_2 _returnvalue_3) false false)
                (else
                  (bind _returnvalue_4 (- (* _from_0_to_1_in_2_sec -45.0) 45.0))
                  (`SceneComponent.K2_SetRelativeRotation` _camera (`KismetMathLibrary.MakeRotator` 0.0 _returnvalue_4 _returnvalue_3) false false)))
              (elif (`self.CamRotUp`)
                (bind _returnvalue_5 (- (* (stale `Key|NumPadFour` _from_0_to_1_in_2_sec) 45.0) 45.0))
                (`SceneComponent.K2_SetRelativeRotation` _camera (`KismetMathLibrary.MakeRotator` 0.0 _returnvalue_2 _returnvalue_5) false false)
                (else
                  (`SceneComponent.K2_SetRelativeRotation` _camera (`KismetMathLibrary.MakeRotator` 0.0 _returnvalue_4 _returnvalue_5) false false))))
            (elif (`self.CamRotUp`)
              (`SceneComponent.K2_SetRelativeRotation` _camera (`KismetMathLibrary.MakeRotator` 0.0 _returnvalue_2 _yaw) false false)
              (else
                (`SceneComponent.K2_SetRelativeRotation` _camera (`KismetMathLibrary.MakeRotator` 0.0 _returnvalue_4 _yaw) false false)))))
        (:`Finished`
          (if (`self.CamYReturn`)
            (if (`self.CamRotDown`)
              (set `self.CamRotDown` false)
              (if (`PlayerController.IsInputKeyDown` _returnvalue Key)
                (goto _label)
                (else
                  (set `self.CamYReturn` false :!label _label_4)))
              (else
                (set `self.CamRotUp` false)
                (if (`PlayerController.IsInputKeyDown` _returnvalue (stale `Key|NumPadTwo` Key))
                  (if (not (`self.CamRotUp`)) :!label _label_5
                    (set `self.CamRotDown` true)
                    (goto _label_2))
                  (else
                    (goto _label_4))))))))))
  (:`Released`
    (set `self.CamYReturn` true :!label _label_6)
    (goto _label_2 :!via `Reverse`)))

(event `Key|NumPadTwo`
  (params (Key :type "Key Structure"))
  ;[1 1 1] Camera rotation (not perfect but good enough)
  ;;[1 1 1] Camera Up and Down rotation
  (:`Pressed`
    (goto _label_5))
  (:`Released`
    (goto _label_6)))

(event `Key|NumPadFour`
  (params (Key :type "Key Structure"))
  (bind _returnvalue (`GameplayStatics.GetPlayerController` 0))
  (bind _camera (`self.Camera`))
  (bind _pitch (.pitch (.rotation (`SceneComponent.GetRelativeTransform` _camera))))
  ;[1 1 1] Camera rotation (not perfect but good enough)
  ;;[1 1 1] Camera Left and Right rotation
  (:`Pressed`
    (if (not (`self.CamRotRight`)) :!label _label_7
      (set `self.CamRotLeft` true)
      (bind (_direction _from_0_to_1_in_2_sec) (`Timeline|TimelineZAxis` :!label _label_8)
        (:`Update`
          ;;[1 1 1] Check if movement is exclusive
          (if (or (`self.CamRotUp`) (`self.CamRotDown`))
            (goto _label_3)
            (else
              ;;[1 1 1] Apply movment
              (if (`self.CamRotLeft`)
                (`SceneComponent.K2_SetRelativeRotation` _camera (`KismetMathLibrary.MakeRotator` 0.0 _pitch (- (* _from_0_to_1_in_2_sec -45.0) 45.0)) false false)
                (else
                  (`SceneComponent.K2_SetRelativeRotation` _camera (`KismetMathLibrary.MakeRotator` 0.0 _pitch (- (* _from_0_to_1_in_2_sec 45.0) 45.0)) false false))))))
        (:`Finished`
          (if (`self.CamZReturn`)
            (if (`self.CamRotRight`)
              (set `self.CamRotRight` false)
              (if (`PlayerController.IsInputKeyDown` _returnvalue Key)
                (goto _label_7)
                (else
                  (set `self.CamZReturn` false :!label _label_9)))
              (else
                (set `self.CamRotLeft` false)
                (if (`PlayerController.IsInputKeyDown` _returnvalue (stale `Key|NumPadSix` Key))
                  (if (not (`self.CamRotLeft`)) :!label _label_10
                    (set `self.CamRotRight` true)
                    (goto _label_8))
                  (else
                    (goto _label_9))))))))))
  (:`Released`
    (set `self.CamZReturn` true :!label _label_11)
    (goto _label_8 :!via `Reverse`)))

(event `Key|NumPadSix`
  (params (Key :type "Key Structure"))
  ;[1 1 1] Camera rotation (not perfect but good enough)
  ;;[1 1 1] Camera Left and Right rotation
  (:`Pressed`
    (goto _label_10))
  (:`Released`
    (goto _label_11)))

(fn `UserConstructionScript`)